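; BP_Monster1 is an enemy that chases the player, takes weapon hits and drops experience on death.
; On BeginPlay it copies mesh and stats from STMonsterV; Tick turns it toward the player and offsets it horizontally by MonsterSpeed, without delta-time scaling.
; A BP_Weapon capsule overlap applies knockback away from the player and subtracts WeaponDamage.
; At zero HP it spawns BP_Exp, leaves the spawner's AllMonster list and destroys itself.
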(event OnComponentBeginOverlap(CapsuleComponent)
  (params (OverlappedComponent :type Primitive%20Component%20Object%20Reference) (OtherActor :type Actor%20Object%20Reference) (OtherComp :type Primitive%20Component%20Object%20Reference) (OtherBodyIndex :type Integer) (bFromSweep :type Boolean) (SweepResult :type Hit%20Result%20Structure%20%28by%20ref%29))
  (bind _returnvalue (Game|GetPlayerCharacter 0))
  (bind _returnvalue_2 (Transformation|GetActorLocation))
  (bind _capsulecomponent (Variables|Collision|GetCapsuleComponent))
  (bind _returnvalue_3 (Transformation|GetWorldLocation _capsulecomponent))
  (bind _returnvalue_4 (Transformation|GetActorLocation _returnvalue))
  (bind _returnvalue_5 (Math|Rotator|FindLookatRotation _returnvalue_4 _returnvalue_2))
  (bind _returnvalue_6 (Math|Vector|GetForwardVector _returnvalue_5))
  (bind _returnvalue_7 (* _returnvalue_6 1.5e+02))
  ;[1 1 1] 몬스터 피해시 MonsterHp 감소, 0 이하 시 파괴, 파괴 시 ExpPoint 스폰
  (bind _asbp_weapon (Utilities|Casting|CastToBP_Weapon OtherActor))
  (Physics|AddImpulse (Variables|Collision|GetCapsuleComponent) (Math|Vector|MakeVector (.x _returnvalue_7) (.y _returnvalue_7) 0.0) "None" true)
  (Development|PrintString (Utilities|String|ToString(Float) (Variables|/Game/VSPProject/VSP_BluePrint/Weapon/BP_Weapon.BP_Weapon_C|GetWeapon_Damage _asbp_weapon)))
  (bind _output_get (Variables|Default|SetMonsterHp (- (Variables|Default|GetMonsterHp) (Variables|/Game/VSPProject/VSP_BluePrint/Weapon/BP_Weapon.BP_Weapon_C|GetWeapon_Damage _asbp_weapon))))
  (if (<= _output_get 0.0)
    (Game|SpawnActorfromClass "/Game/VSPProject/VSP_BluePrint/BP_Exp.BP_Exp_C" (Math|Transform|MakeTransform (Math|Vector|MakeVector (.x _returnvalue_3) (.y _returnvalue_3) (- (.z _returnvalue_3) 79.0)) "0, 0, 0" "1,1,1") "Undefined" 0 0)
    (Utilities|FlowControl|Sequence
      (:then_0
        (Utilities|Array|RemoveItem (Variables|/Game/VSPProject/VSP_BluePrint/BP_MonsterSpawner.BP_MonsterSpawner_C|GetAllMonster (Variables|Default|GetMonsterSpawnerRef)) self))
      (:then_1
        (Actor|DestroyActor)))))

(event EventBeginPlay
  (bind _st_monsterv (Variables|Default|GetST_MonsterV))
  ;[1 1 1] Target에 정보 넣어주기
  (Variables|Default|SetTarget (Game|GetPlayerCharacter 0))
  ;[1 1 1] ST_MonsterV를 호출해서 각 값에 저장
  (Class|SkinnedMeshComponent|SetSkeletalMesh (Variables|Character|GetMesh) (.mesh _st_monsterv) true)
  (Variables|Default|SetMonsterHp (.hp _st_monsterv))
  (Variables|Default|SetMonsterSpeed (.speed _st_monsterv))
  (Variables|Default|SetMonsterDamage (.damage _st_monsterv))
  (Variables|Default|SetMonsterExp (.exp _st_monsterv)))

(event EventTick
  (params (DeltaSeconds :type Float%20%28single-precision%29))
  (bind _returnvalue (Transformation|GetActorLocation))
  (bind _returnvalue_2 (Transformation|GetActorLocation))
  (bind _target (Variables|Default|GetTarget))
  (bind _target_2 (Variables|Default|GetTarget))
  (bind _monsterspeed (Variables|Default|GetMonsterSpeed))
  (bind _returnvalue_3 (Transformation|GetActorLocation _target))
  (bind _returnvalue_4 (Transformation|GetActorLocation _target_2))
  (bind _returnvalue_5 (Math|Rotator|FindLookatRotation _returnvalue_2 _returnvalue_4))
  (bind _returnvalue_6 (Math|Rotator|FindLookatRotation _returnvalue _returnvalue_3))
  (bind _returnvalue_7 (Math|Vector|GetForwardVector _returnvalue_6))
  ;[1 1 1] 몬스터가 플레이어를 따라가기
  (Transformation|SetActorRotation (Math|Rotator|MakeRotator (.roll _returnvalue_5) 0.0 (.yaw _returnvalue_5)))
  (Transformation|AddActorWorldOffset (Math|Vector|MakeVector (* _monsterspeed (.x _returnvalue_7)) (* _monsterspeed (.y _returnvalue_7)) 0.0)))

(fn ConstructionScript)