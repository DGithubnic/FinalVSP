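; Auto-firing magic wand weapon that shoots BP_MagicBullet projectiles from the player at the nearest BP_Monster1.
; On BeginPlay it registers with BP_Player and loads its DT_Weapon stats.
; Tick interval serves as cooldown: each tick box-traces a fixed world area and spawns bullets by WeaponCount.
; Upgrade events adjust count, cooldown and speed using player passives; speed-up replaces the table speed with a hardcoded base.
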(event Custom|MagicWand_CoolTimeUp_E
  ;[1 1 1] CoolTime Up
  (Actor|Tick|SetActorTickInterval (- (Variables|Default|GetWeapon_CoolTime) (Variables|/Game/VSPProject/VSP_BluePrint/Weapon/BP_Passive.BP_Passive_C|GetPassive_CoolTime (Variables|/Game/VSPProject/VSP_BluePrint/BP_Player.BP_Player_C|GetPlayer_PassiveRef (stale EventBeginPlay _asbp_player))))))

(event Custom|MagicWand_Add_E
  ;[1 1 1] Level Up
  (Variables|Default|SetWeapon_Count (+ (Variables|Default|GetWeapon_Count) 1)))

(event Custom|MagicWand_SpeedUp_E
  ;[1 1 1] Speed Up
  (bind _output_get (Variables|Default|SetWeapon_Speed 7e+01))
  (Variables|Default|SetWeapon_Speed (+ _output_get (* (Variables|/Game/VSPProject/VSP_BluePrint/Weapon/BP_Passive.BP_Passive_C|GetPassive_Speed (Variables|/Game/VSPProject/VSP_BluePrint/BP_Player.BP_Player_C|GetPlayer_PassiveRef (stale EventBeginPlay _asbp_player))) 6e+01))))

(event EventBeginPlay
  ;[1 1 1] Player 매개체에 형변환, DT에 연동
  (bind _asbp_player (Utilities|Casting|CastToBP_Player (Game|GetPlayerCharacter 0)))
  (Variables|/Game/VSPProject/VSP_BluePrint/BP_Player.BP_Player_C|SetPlayer_MagicWandRef _asbp_player self)
  (bind _returnvalue (Utilities|GetDataTableRow "/Game/VSPProject/VSP_Struct/DT_Weapon.DT_Weapon" "MagicWand")
    (:then
      (Variables|Default|SetWeapon_CoolTime (.cooltime _returnvalue))
      (Variables|Default|SetWeapon_Count (.weaponcount _returnvalue))
      (Variables|Default|SetWeapon_Speed (.speed _returnvalue))
      (CallFunction|MagicWandSpeedUpE)
      (CallFunction|MagicWandCoolTimeUpE))))

(event Collision|EventActorBeginOverlap
  (params (OtherActor :type Actor%20Object%20Reference))
  ;[1 1 1] 폐기한 노드
  ;;[1 1 1] 이후에 컴포넌트
)

(event EventTick
  (params (DeltaSeconds :type Float%20%28single-precision%29))
  ;[1 1 1] 거리 계산 후 Near 타겟 지정 후 Bullet Spawn
  (bind (_outhits _returnvalue) (Class|KismetSystemLibrary|BoxTraceMulti "0, 0,20.000000" "0, 0, 0" "5100.000000,1400.000000,70.000000" "0, 0, 0" "TraceTypeQuery1" false (Utilities|Array|MakeArray (Game|GetPlayerController 0)) "ForDuration" true))
  (if _returnvalue
    (Utilities|Array|Clear (Variables|Default|GetMagicWand_AllMonster))
    (for _array_element _outhits
      (bind _asbp_monster_1 (Utilities|Casting|CastToBP_Monster1 (.HitActor (Collision|BreakHitResult _array_element))))
      (Utilities|Array|AddUnique (Variables|Default|GetMagicWand_AllMonster) _asbp_monster_1))
    (bind _output_get (Variables|Default|SetMagicWand_TargetMonster (.ReturnValue (Actor|FindNearestActor (Transformation|GetActorLocation (Game|GetPlayerCharacter 0)) (Variables|Default|GetMagicWand_AllMonster)))))
    (Utilities|IsValid _output_get
      (:Is%20Valid
        (for _index (range 0 (Variables|Default|GetWeapon_Count))
          (Game|SpawnActorfromClass "/Game/VSPProject/VSP_BluePrint/Weapon/MagicWand/BP_MagicBullet.BP_MagicBullet_C" (Math|Transform|MakeTransform (Transformation|GetActorLocation (Game|GetPlayerCharacter 0)) "0, 0, 0" "1,1,1") "Undefined" 0 _output_get (Variables|Default|GetWeapon_Speed) 0))))))

(fn ConstructionScript
  (|CallParentFunction))