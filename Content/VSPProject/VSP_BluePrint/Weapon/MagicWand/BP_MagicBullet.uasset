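; Magic wand projectile that launches itself toward its BulletTarget when play begins.
; On BeginPlay it detaches its Sphere component, keeping the world transform, and applies a one-time impulse to it.
; The impulse direction comes from a look-at rotation between player character 0 and the target, not from the bullet's own position.
; Only the scaled X and Y of that direction are fed in, so the launch ignores height difference.
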(event EventBeginPlay
  (bind _returnvalue (Game|GetPlayerCharacter 0))
  (bind _bullet_target (Variables|Default|GetBullet_Target))
  (bind _returnvalue_2 (Transformation|GetActorLocation _bullet_target))
  (bind _returnvalue_3 (Transformation|GetActorLocation _returnvalue))
  (bind _returnvalue_4 (Math|Rotator|FindLookatRotation _returnvalue_3 _returnvalue_2))
  (bind _returnvalue_5 (Math|Vector|GetForwardVector _returnvalue_4))
  (bind _returnvalue_6 (* _returnvalue_5 1e+02))
  (Transformation|DetachFromComponent (Variables|Default|GetSphere) "KeepWorld" "KeepWorld" "KeepWorld" true)
  (Physics|AddImpulse (Variables|Default|GetSphere) (Math|Vector|MakeVector (.x _returnvalue_6) (.y _returnvalue_6) 0.0) "None" false))

(fn ConstructionScript
  (|CallParentFunction))