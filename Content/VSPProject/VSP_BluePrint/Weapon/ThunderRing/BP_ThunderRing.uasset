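; BP_ThunderRing is a player weapon that periodically strikes random nearby monsters with lightning.
; BeginPlay registers it with BP_Player and loads DT_Weapon stats, then cooldown and scale events override those values using player passives.
; Tick, with its interval as cooldown, sphere-traces for unique BP_Monster1 actors, spawning effects and short-lived sphere components at randomly picked ones.
; Damage is loaded but not applied here; a level-up event raises the strike count.
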(event Custom|ThunderRing_CoolTimeUp_E
  ;[1 1 1] CoolTime Up
  (Variables|Default|SetWeapon_CoolTime 7.0)
  (Variables|Default|SetWeapon_CoolTime (- (Variables|Default|GetWeapon_CoolTime) (Variables|/Game/VSPProject/VSP_BluePrint/Weapon/BP_Passive.BP_Passive_C|GetPassive_CoolTime (Variables|/Game/VSPProject/VSP_BluePrint/BP_Player.BP_Player_C|GetPlayer_PassiveRef (stale EventBeginPlay _asbp_player)))))
  (Actor|Tick|SetActorTickInterval (Variables|Default|GetWeapon_CoolTime)))

(event Custom|ThunderRing_Add_E
  ;[1 1 1] Level Up
  (Variables|Default|SetWeapon_Count (+ (Variables|Default|GetWeapon_Count) 1)))

(event Custom|ThunderRing_ScaleUp_E
  ;[1 1 1] Scale Up
  (Variables|Default|SetWeapon_Scale "1.000000,1.000000,1.000000")
  (Variables|Default|SetWeapon_Scale (* (Variables|Default|GetWeapon_Scale) (* (Variables|/Game/VSPProject/VSP_BluePrint/Weapon/BP_Passive.BP_Passive_C|GetPassive_Scale (Variables|/Game/VSPProject/VSP_BluePrint/BP_Player.BP_Player_C|GetPlayer_PassiveRef (stale EventBeginPlay _asbp_player))) 3.0))))

(event EventBeginPlay
  ;[1 1 1] Player 매개체에 형변환, DT에 연동
  (bind _asbp_player (Utilities|Casting|CastToBP_Player (Game|GetPlayerCharacter 0)))
  (Variables|/Game/VSPProject/VSP_BluePrint/BP_Player.BP_Player_C|SetPlayer_ThunderRingRef _asbp_player self)
  ;;[1 1 1] 첫 쿨타임
  (Actor|Tick|SetActorTickInterval (Variables|Default|GetWeapon_CoolTime))
  (bind _returnvalue (Utilities|GetDataTableRow "/Game/VSPProject/VSP_Struct/DT_Weapon.DT_Weapon" "ThunderRing")
    (:then
      (Variables|Default|SetWeapon_Damage (.damage _returnvalue))
      (Variables|Default|SetWeapon_CoolTime (.cooltime _returnvalue))
      (Variables|Default|SetWeapon_Scale (.scale _returnvalue))
      (Variables|Default|SetWeapon_Count (.weaponcount _returnvalue))
      (CallFunction|ThunderRingCoolTimeUpE)
      (CallFunction|ThunderRingScaleUpE))))

(event EventTick
  (params (DeltaSeconds :type Float%20%28single-precision%29))
  (bind _returnvalue (Transformation|GetActorLocation))
  ;[1 1 1] 범위 내 몬스터 중복 제거하여 배열로 초기화 한 후에 랜덤 타겟에 콜리전과 이펙트 생성
  (bind (_outhits _returnvalue_2) (Collision|MultiSphereTraceByChannel _returnvalue (+ _returnvalue 0.01) 1e+03 "TraceTypeQuery1" false (Utilities|Array|MakeArray (Game|GetPlayerCharacter 0)) "ForDuration" true "(R=1.000000,G=0.000000,B=0.000000,A=1.000000)" "(R=0.000000,G=1.000000,B=0.000000,A=1.000000)" 3.0))
  (if _returnvalue_2
    (Utilities|Array|Clear (Variables|Default|GetThunderRing_AllMonster))
    (for _array_element _outhits
      (bind _asbp_monster_1 (Utilities|Casting|CastToBP_Monster1 (.HitActor (Collision|BreakHitResult _array_element))))
      (Utilities|Array|AddUnique (Variables|Default|GetThunderRing_AllMonster) _asbp_monster_1))
    (for _index (range 0 (Variables|Default|GetWeapon_Count))
      (if (Utilities|Array|IsValidIndex (Variables|Default|GetThunderRing_AllMonster))
        (bind _output_get (Variables|Default|SetThunderRing_TargetMonster (.OutItem (Utilities|Array|Random (Variables|Default|GetThunderRing_AllMonster)))))
        (Utilities|Array|RemoveItem (Variables|Default|GetThunderRing_AllMonster) _output_get)
        (Effects|SpawnEmitteratLocation "/Game/FXVarietyPack/Particles/LightningRing.LightningRing" (Transformation|GetActorLocation _output_get) "0, 0, 0" (* (+ (Variables|Default|GetWeapon_Scale) 1.0) 0.2))
        (bind _returnvalue_3 (AddComponent|AddSphereComponent true (Math|Transform|MakeTransform (Transformation|GetActorLocation _output_get) "0, 0, 0" (Variables|Default|GetWeapon_Scale))))
        (Transformation|AttachComponentToComponent _returnvalue_3 0 "None" "KeepRelative" "KeepRelative" "KeepRelative" true)
        (Utilities|Array|Add (Variables|Default|GetThunderRing_Remove) _returnvalue_3)))
    (Utilities|FlowControl|Delay 0.3)
    (for _array_element_2 (Variables|Default|GetThunderRing_Remove)
      (Utilities|IsValid _array_element_2
        (:Is%20Valid
          (Components|DestroyComponent _array_element_2))))))

(fn ConstructionScript
  (|CallParentFunction))