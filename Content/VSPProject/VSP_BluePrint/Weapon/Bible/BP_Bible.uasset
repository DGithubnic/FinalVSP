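; Orbiting Bible weapon that registers itself with BP_Player and loads its stats from DT_Weapon.
; Tick yaws the root, revolving runtime-added static mesh and box component pairs stored in parallel arrays.
; Bible_Add_E adds a pair on level-up and re-spaces all evenly around the circle.
; Speed and scale events recompute spin rate and orbit radius from hardcoded bases plus player passives, replacing the table values at BeginPlay.
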(event Custom|Bible_Add_E
  (bind _bible_array (Variables|Default|GetBible_Array))
  (bind _bible_cbarray (Variables|Default|GetBible_CBArray))
  ;[1 1 1] Bible, Bible_CB 추가 후 위치 재조정
  ;;[1 1 1] 레벨업시 호출
  (Utilities|FlowControl|Sequence
    (:then_0
      (bind _returnvalue (AddComponent|AddStaticMeshComponent false (Math|Transform|MakeTransform "0, 0, 0" "0,0.000000, 0" "1,1,1")))
      (Utilities|Array|Add (Variables|Default|GetBible_Array) _returnvalue)
      (Transformation|AttachComponentToComponent _returnvalue 0 "None" "KeepRelative" "KeepRelative" "KeepRelative" true)
      (for (_array_element _array_index) _bible_array
        (Transformation|SetRelativeLocationAndRotation _array_element (Math|Vector|RotateVectorAroundAxis (Math|Vector|MakeVector (.x (Variables|Default|GetWeapon_Scale)) 0.0 0.0) (Math|Conversions|ToFloat(Integer) (* (+ _array_index 1) (/ 360 (+ (Utilities|Array|LastIndex _bible_array) 1)))) "0, 0,1.000000") (Math|Rotator|MakeRotator 0.0 0.0 (Math|Conversions|ToFloat(Integer) (* (+ _array_index 1) (/ 360 (+ (Utilities|Array|LastIndex _bible_array) 1))))) false false)))
    (:then_1
      (bind _returnvalue_2 (AddComponent|AddBoxComponent false (Math|Transform|MakeTransform "0, 0, 0" "0, 0, 0" "1.500000,1.500000,1.500000")))
      (Utilities|Array|Add (Variables|Default|GetBible_CBArray) _returnvalue_2)
      (Transformation|AttachComponentToComponent _returnvalue_2 0 "None" "KeepRelative" "KeepRelative" "KeepRelative" true)
      (for (_array_element_2 _array_index_2) _bible_cbarray
        (Transformation|SetRelativeLocation _array_element_2 (Math|Vector|RotateVectorAroundAxis (Math|Vector|MakeVector (.x (Variables|Default|GetWeapon_Scale)) 0.0 0.0) (Math|Conversions|ToFloat(Integer) (* (+ _array_index_2 1) (/ 360 (+ (Utilities|Array|LastIndex _bible_cbarray) 1)))) "0, 0,1.000000") false false)))))

(event Custom|Bible_ScaleUp_E
  (bind _bible_cbarray (Variables|Default|GetBible_CBArray))
  (bind _bible_array (Variables|Default|GetBible_Array))
  ;[1 1 1] ScaleUp 시에 위치 재조정
  (Variables|Default|SetWeapon_Scale (Math|Vector|MakeVector 2e+02 0.0 0.0))
  (Variables|Default|SetWeapon_Scale (Math|Vector|MakeVector (+ (.x (Variables|Default|GetWeapon_Scale)) (* (Variables|/Game/VSPProject/VSP_BluePrint/Weapon/BP_Passive.BP_Passive_C|GetPassive_Scale (Variables|/Game/VSPProject/VSP_BluePrint/BP_Player.BP_Player_C|GetPlayer_PassiveRef (stale EventBeginPlay _asbp_player))) 5e+01)) 0.0 0.0))
  (Utilities|FlowControl|Sequence
    (:then_0
      (for (_array_element _array_index) _bible_array
        (Transformation|SetRelativeLocation _array_element (Math|Vector|RotateVectorAroundAxis (Math|Vector|MakeVector (.x (Variables|Default|GetWeapon_Scale)) 0.0 0.0) (Math|Conversions|ToFloat(Integer) (* (+ _array_index 1) (/ 360 (+ (Utilities|Array|LastIndex _bible_array) 1)))) "0, 0,1.000000") false false)))
    (:then_1
      (for (_array_element_2 _array_index_2) _bible_cbarray
        (Transformation|SetRelativeLocation _array_element_2 (Math|Vector|RotateVectorAroundAxis (Math|Vector|MakeVector (.x (Variables|Default|GetWeapon_Scale)) 0.0 0.0) (Math|Conversions|ToFloat(Integer) (* (+ _array_index_2 1) (/ 360 (+ (Utilities|Array|LastIndex _bible_cbarray) 1)))) "0, 0,1.000000") false false)))))

(event Custom|Bible_SpeedUp_E
  ;[1 1 1] SpeedUp
  (Variables|Default|SetWeapon_Speed 7e+01)
  (Variables|Default|SetWeapon_Speed (+ (Variables|Default|GetWeapon_Speed) (* (Variables|/Game/VSPProject/VSP_BluePrint/Weapon/BP_Passive.BP_Passive_C|GetPassive_Speed (Variables|/Game/VSPProject/VSP_BluePrint/BP_Player.BP_Player_C|GetPlayer_PassiveRef (stale EventBeginPlay _asbp_player))) 3e+01))))

(event EventBeginPlay
  ;[1 1 1] Player에 정보 넣어주기
  (bind _asbp_player (Utilities|Casting|CastToBP_Player (Game|GetPlayerCharacter 0)))
  (Variables|/Game/VSPProject/VSP_BluePrint/BP_Player.BP_Player_C|SetPlayer_BibleRef _asbp_player self)
  ;[1 1 1] DT 연동
  (bind _returnvalue (Utilities|GetDataTableRow "/Game/VSPProject/VSP_Struct/DT_Weapon.DT_Weapon" "Bible")
    (:then
      (Variables|Default|SetWeapon_Damage (.damage _returnvalue))
      (Variables|Default|SetWeapon_Speed (.speed _returnvalue))
      (Variables|Default|SetWeapon_Scale (.scale _returnvalue))
      ;[1 1 1] 첫 Bible, Bible_CB 소환 (하나의 블루프린트에 Static Mesh Component 추가로 같은 스태틱 매쉬를 계속해서 소환 할 수 있다.)
      (Utilities|FlowControl|Sequence
        (:then_0
          (bind _returnvalue_2 (AddComponent|AddStaticMeshComponent false (Math|Transform|MakeTransform (Math|Vector|MakeVector (.x (Variables|Default|GetWeapon_Scale)) 0.0 0.0) "0,0.000000, 0" "1,1,1")))
          (Utilities|Array|Add (Variables|Default|GetBible_Array) _returnvalue_2)
          (Transformation|AttachComponentToComponent _returnvalue_2 0 "None" "KeepRelative" "KeepRelative" "KeepRelative" true))
        (:then_1
          (bind _returnvalue_3 (AddComponent|AddBoxComponent false (Math|Transform|MakeTransform (Math|Vector|MakeVector (.x (Variables|Default|GetWeapon_Scale)) 0.0 0.0) "0,0.000000, 0" "1.500000,1.500000,1.500000")))
          (Utilities|Array|Add (Variables|Default|GetBible_CBArray) _returnvalue_3)
          (Transformation|AttachComponentToComponent _returnvalue_3 0 "None" "KeepRelative" "KeepRelative" "KeepRelative" true)
          (CallFunction|BibleScaleUpE)
          (CallFunction|BibleSpeedUpE))))))

(event EventTick
  (params (DeltaSeconds :type Float%20%28single-precision%29))
  ;[1 1 1] Bible 공전 (원래 Axis를 썼지만 위처럼 캐릭터)
  (bind _output_get (Variables|Default|SetBible_Rotation (+ (* (* DeltaSeconds -1.0) (Variables|Default|GetWeapon_Speed)) (Variables|Default|GetBible_Rotation))))
  (Transformation|SetWorldRotation (Variables|Default|GetDefaultSceneRoot) (Math|Rotator|MakeRotator 0.0 0.0 _output_get) false false))

(fn ConstructionScript)