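; BP_Passive holds the player's passive stats for speed, cooldown and scale.
; On BeginPlay it registers itself as the player's PlayerPassiveRef on BP_Player and loads starting values from the "Passive" row of DT_Passive.
; Three custom events each raise one stat by a flat increment, including cooldown, which increases rather than shrinks.
; The file only stores these values and does not apply them to gameplay.
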(event Custom|Passive_SpeedUp_E
  ;[1 1 1] Passive Speed Up
  (Variables|Default|SetPassive_Speed (+ (Variables|Default|GetPassive_Speed) 1.0)))

(event Custom|Passive_CoolTimeUp_E
  ;[1 1 1] Passive CoolTime Up
  (Variables|Default|SetPassive_CoolTime (+ (Variables|Default|GetPassive_CoolTime) 1.0)))

(event Custom|Passive_ScaleUp_E
  ;[1 1 1] Passive Scale Up
  (Variables|Default|SetPassive_Scale (+ (Variables|Default|GetPassive_Scale) 1.0)))

(event EventBeginPlay
  ;[1 1 1] Player 매개체에 형변환, DT에 연동
  (bind _asbp_player (Utilities|Casting|CastToBP_Player (Game|GetPlayerCharacter 0)))
  (Variables|/Game/VSPProject/VSP_BluePrint/BP_Player.BP_Player_C|SetPlayer_PassiveRef _asbp_player self)
  (bind _returnvalue (Utilities|GetDataTableRow "/Game/VSPProject/VSP_Struct/DT_Passive.DT_Passive" "Passive")
    (:then
      (Variables|Default|SetPassive_Speed (.speed _returnvalue))
      (Variables|Default|SetPassive_CoolTime (.cooltime _returnvalue))
      (Variables|Default|SetPassive_Scale (.scale _returnvalue)))))

(fn ConstructionScript)