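; Monster spawner actor that runs looping timed waves of BP_Monster1 and registers itself with BP_Player at BeginPlay.
; Each wave can raise MonsterLevel up to a cap, then reads that level's DT_Monster row to spawn a batch, with boss levels scaled up.
; Spawn points are re-rolled until far enough from the player.
; Spawned monsters are tracked in AllMonster, whose count prints on Tick.
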(event EventTick
  (params (DeltaSeconds :type Float%20%28single-precision%29))
  (Development|PrintString (Utilities|String|ToString(Integer) (Utilities|Array|Length (Variables|Default|GetAllMonster))) true false "(R=0.000000,G=0.660000,B=1.000000,A=1.000000)" 0.0))

(event EventBeginPlay
  ;[1 1 1] SpawnMonster 함수를 호출
  (Utilities|Time|SetTimerbyFunctionName 0 "SpawnMonster_F" 3.0 true)
  (bind _asbp_player (Utilities|Casting|CastToBP_Player (Game|GetPlayerCharacter 0)))
  (Variables|/Game/VSPProject/VSP_BluePrint/BP_Player.BP_Player_C|SetPlayer_MonsterSpawnerRef _asbp_player self))

(fn ConstructionScript)

(fn SpawnMonsterF
  ;[1 1 1] 몬스터 소환
  (Variables|Default|SetSpawnTime (+ (Variables|Default|GetSpawnTime) 3))
  (if (== (Math|Integer|%(Integer) (Variables|Default|GetSpawnTime) 3) 0)
    (if (== (Variables|Default|GetMonsterLevel) 10)
      _
      (else
        (Math|Integer|IncrementInt (Variables|Default|GetMonsterLevel)
          (:%20%20
            _)))))
  (for _index (range 0 4)
    (bind _returnvalue (Utilities|GetDataTableRow "/Game/VSPProject/VSP_Struct/DT_Monster.DT_Monster" (Utilities|String|StringToName (Utilities|String|ToString(Integer) (Variables|Default|GetMonsterLevel))))
      (:then
        (bind _output_get (Variables|Default|SetMonsterPosition (Math|Vector|MakeVector (Math|Random|RandomFloatinRange -5e+03 5e+03) (Math|Random|RandomFloatinRange -1.5e+03 1.5e+03) 6e+01) :!label _label))
        (if (< 1.8e+03 (Math|Vector|Distance(Vector) _output_get (Transformation|GetActorLocation (Game|GetPlayerCharacter 0))))
          (if (or (== (Variables|Default|GetMonsterLevel) 10) (== (Variables|Default|GetMonsterLevel) 5))
            ;[1 1 1] 보스 몬스터 스케일
            (bind _returnvalue_2 (Game|SpawnActorfromClass "/Game/VSPProject/VSP_BluePrint/BP_Monster1.BP_Monster1_C" (Math|Transform|MakeTransform (Variables|Default|GetMonsterPosition) "0, 0, 0" "2.000000,2.000000,2.000000") "Undefined" 0 _returnvalue self 0))
            ;[1 1 1] 전체 몬스터 배열로 관리
            (bind _returnvalue_3 (Utilities|Array|Add (Variables|Default|GetAllMonster) _returnvalue_2))
            (Variables|Default|SetAllMonsterIndex _returnvalue_3)
            (else
              ;[1 1 1] 일반 몬스터 스케일
              (bind _returnvalue_4 (Game|SpawnActorfromClass "/Game/VSPProject/VSP_BluePrint/BP_Monster1.BP_Monster1_C" (Math|Transform|MakeTransform (Variables|Default|GetMonsterPosition) "0, 0, 0" "1,1,1") "Undefined" 0 _returnvalue self 0))
              ;[1 1 1] 전체 몬스터 배열로 관리
              (bind _returnvalue_5 (Utilities|Array|Add (Variables|Default|GetAllMonster) _returnvalue_4))
              (Variables|Default|SetAllMonsterIndex _returnvalue_5)))
          (else
            (goto _label)))))))